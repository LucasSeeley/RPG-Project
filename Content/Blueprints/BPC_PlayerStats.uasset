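; Actor component that holds the player's health, stamina, XP and level and pushes them to the third-person character's HUD widget.
; It caches the owning BP_ThirdPersonCharacter on BeginPlay, and each stat function writes straight to the matching bar or text.
; DecreaseHealth returns whether health is depleted, and DecreaseStamina refuses costs it cannot cover.
; Reaching max XP raises the level, carries over the excess and scales up the next threshold.
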(event `self.ReceiveBeginPlay`
  (bind _asbp_third_person_character (cast `/Game/ThirdPerson/Blueprints/BP_ThirdPersonCharacter` (`self.GetOwner`)))
  (set `self.Player Character BP` _asbp_third_person_character))

(event `Create Player HUD`
  (bind _returnvalue (/ (`self.Current Health`) (`self.Max Health`)))
  (bind _hud_widget (`/Game/ThirdPerson/Blueprints/BP_ThirdPersonCharacter.HUD Widget` (`self.Player Character BP`)))
  ;[0.05127 0.05127 0.05127] Set HUD Values
  (`ProgressBar.SetPercent` (`/Game/UI/WB_HUD.HealthBar` _hud_widget) _returnvalue)
  (`TextBlock.SetText` (`/Game/UI/WB_HUD.HealthText` _hud_widget) (`KismetTextLibrary.AsPercent_Float` _returnvalue "HalfToEven"))
  (`ProgressBar.SetPercent` (`/Game/UI/WB_HUD.StaminaBar` _hud_widget) (/ (`self.Current Stamina`) (`self.Max Stamina`)))
  (set `TextBlock.Text` (`KismetTextLibrary.Conv_IntToText` (`self.Level`)) (`/Game/UI/WB_HUD.LevelText` _hud_widget))
  (`ProgressBar.SetPercent` (`/Game/UI/WB_HUD.XPBar` _hud_widget) (/ (`self.XP`) (`self.Max XP`))))

(fn `Decrease Health`
  (params (Damage :type "Float (double-precision)"))
  (returns (`isPlayerDead?` :type Boolean))
  (bind _hud_widget (`/Game/ThirdPerson/Blueprints/BP_ThirdPersonCharacter.HUD Widget` (`self.Player Character BP`)))
  (bind _output_get (set `self.Current Health` (- (`self.Current Health`) Damage)))
  (bind _returnvalue (/ _output_get (`self.Max Health`)))
  (`ProgressBar.SetPercent` (`/Game/UI/WB_HUD.HealthBar` _hud_widget) _returnvalue)
  (`TextBlock.SetText` (`/Game/UI/WB_HUD.HealthText` _hud_widget) (`KismetTextLibrary.AsPercent_Float` _returnvalue "HalfToEven"))
  (return (<= _output_get 0.0)))

(fn `Decrease Stamina`
  (params (`Stamina Depleted` :type "Float (double-precision)"))
  (returns (`Action Performed?` :type Boolean))
  (bind _returnvalue (- (`self.Current Stamina`) `Stamina Depleted`))
  (if (>= _returnvalue 0.0)
    (bind _output_get (set `self.Current Stamina` _returnvalue))
    (`ProgressBar.SetPercent` (`/Game/UI/WB_HUD.StaminaBar` (`/Game/ThirdPerson/Blueprints/BP_ThirdPersonCharacter.HUD Widget` (`self.Player Character BP`))) (/ _output_get (`self.Max Stamina`)))
    (return true)
    (else
      (return false))))

(fn `Increase Health`
  (params (`Incremental Health` :type "Float (double-precision)"))
  (bind _hud_widget (`/Game/ThirdPerson/Blueprints/BP_ThirdPersonCharacter.HUD Widget` (`self.Player Character BP`)))
  (bind _output_get (set `self.Current Health` (`KismetMathLibrary.FMin` (+ `Incremental Health` (`self.Current Health`)) (`self.Max Health`))))
  (bind _returnvalue (/ _output_get (`self.Max Health`)))
  (`ProgressBar.SetPercent` (`/Game/UI/WB_HUD.HealthBar` _hud_widget) _returnvalue)
  (`TextBlock.SetText` (`/Game/UI/WB_HUD.HealthText` _hud_widget) (`KismetTextLibrary.AsPercent_Float` _returnvalue "HalfToEven")))

(fn `Increase Level`
  (params (`Levels Increased` :type Integer))
  (bind _max_xp (`self.Max XP`))
  (bind _hud_widget (`/Game/ThirdPerson/Blueprints/BP_ThirdPersonCharacter.HUD Widget` (`self.Player Character BP`)))
  (bind _output_get (set `self.Level` (+ `Levels Increased` (`self.Level`))))
  (set `self.XP` (- (`self.XP`) _max_xp))
  (set `self.Max XP` (* _max_xp 1.2))
  (set `TextBlock.Text` (`KismetTextLibrary.Conv_IntToText` _output_get) (`/Game/UI/WB_HUD.LevelText` _hud_widget))
  (`ProgressBar.SetPercent` (`/Game/UI/WB_HUD.XPBar` _hud_widget) (/ (`self.XP`) (`self.Max XP`))))

(fn `Increase Max Health`
  (params (`Incremental Health` :type "Float (double-precision)"))
  (bind _hud_widget (`/Game/ThirdPerson/Blueprints/BP_ThirdPersonCharacter.HUD Widget` (`self.Player Character BP`)))
  (bind _output_get (set `self.Max Health` (+ (`self.Max Health`) `Incremental Health`)))
  (bind _returnvalue (/ (`self.Current Health`) _output_get))
  (`ProgressBar.SetPercent` (`/Game/UI/WB_HUD.HealthBar` _hud_widget) _returnvalue)
  (`TextBlock.SetText` (`/Game/UI/WB_HUD.HealthText` _hud_widget) (`KismetTextLibrary.AsPercent_Float` _returnvalue "HalfToEven")))

(fn `Increase Max Stamina`
  (params (`Incremental Stamina` :type "Float (double-precision)"))
  (bind _output_get (set `self.Max Stamina` (+ (`self.Max Stamina`) `Incremental Stamina`)))
  (`ProgressBar.SetPercent` (`/Game/UI/WB_HUD.StaminaBar` (`/Game/ThirdPerson/Blueprints/BP_ThirdPersonCharacter.HUD Widget` (`self.Player Character BP`))) (/ (`self.Current Stamina`) _output_get)))

(fn `Increase Stamina`
  (params (`Incremental Stamina` :type "Float (double-precision)"))
  (bind _output_get (set `self.Current Stamina` (`KismetMathLibrary.FMin` (+ `Incremental Stamina` (`self.Current Stamina`)) (`self.Max Stamina`))))
  (`ProgressBar.SetPercent` (`/Game/UI/WB_HUD.StaminaBar` (`/Game/ThirdPerson/Blueprints/BP_ThirdPersonCharacter.HUD Widget` (`self.Player Character BP`))) (/ _output_get (`self.Max Stamina`))))

(fn `Increase XP`
  (params (`XP Gained` :type "Float (double-precision)"))
  (bind _max_xp (`self.Max XP`))
  (bind _output_get (set `self.XP` (+ `XP Gained` (`self.XP`))))
  (if (>= _output_get _max_xp)
    (`self.Increase Level` 1)
    (else
      (`ProgressBar.SetPercent` (`/Game/UI/WB_HUD.XPBar` (`/Game/ThirdPerson/Blueprints/BP_ThirdPersonCharacter.HUD Widget` (`self.Player Character BP`))) (/ (`self.XP`) _max_xp)))))