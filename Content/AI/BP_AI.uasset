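; Melee enemy character that fights with a sword combo, takes damage and can be stealth-assassinated from behind.
; Attack calls feed a three-montage combo with buffered follow-ups, while timer-looped or one-shot sphere traces damage "Damageable" actors.
; Damage plays hit reactions, launches the enemy and drains BPCPlayerStats; death ragdolls it and awards player XP.
; Assassination plays a paired victim montage before ragdolling; overlaps toggle its prompt, which faces the camera alongside the HUD widget.
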(event `self.ReceiveBeginPlay`
  (bind _aswb_dummy_hud (cast `/Game/UI/WB_DummyHUD` (`WidgetComponent.GetWidget` (`self.HUD Widget`))))
  (set `self.dummyHUD` _aswb_dummy_hud)
  (`/Game/Blueprints/BPC_PlayerStats.Initialize Stats` (`self.BPC_PlayerStats`)))

(event `Start Sword Trace`
  ;[0.05127 0.05127 0.05127] Sword Trace
  (bind _returnvalue (`KismetSystemLibrary.K2_SetTimerDelegate` (delegate `Sword Trace Loop`) 0.1 true))
  (set `self.swordTraceLoop` _returnvalue))

(event `self.ReceiveTick`
  (params (DeltaSeconds :type "Float (single-precision)"))
  ;[0.05127 0.05127 0.05127] Assassinate Widget Rotation
  (`SceneComponent.K2_SetWorldRotation` (`self.Assassinate Widget`) (`KismetMathLibrary.FindLookAtRotation` (`SceneComponent.K2_GetComponentLocation` (`self.Assassinate Widget`)) (`SceneComponent.K2_GetComponentLocation` (`PlayerCameraManager.TransformComponent` (`GameplayStatics.GetPlayerCameraManager` 0)))) false false)
  (`SceneComponent.K2_SetWorldRotation` (`self.HUD Widget`) (`KismetMathLibrary.FindLookAtRotation` (`SceneComponent.K2_GetComponentLocation` (`self.Assassinate Widget`)) (`SceneComponent.K2_GetComponentLocation` (`PlayerCameraManager.TransformComponent` (`GameplayStatics.GetPlayerCameraManager` 0)))) false false))

(event `Die`
  ;[0.05127 0.05127 0.05127] Die
  (`PrimitiveComponent.SetCollisionObjectType` (`self.Mesh`) "ECC_PhysicsBody")
  (`PrimitiveComponent.SetSimulatePhysics` (`self.Mesh`) true)
  (`CharacterMovementComponent.SetMovementMode` (`self.CharacterMovement`) "MOVE_None" 0)
  (`|ExecutionSequence`
    (:`then_0`
      (bind _asbp_third_person_character (cast `/Game/ThirdPerson/Blueprints/BP_ThirdPersonCharacter` (`GameplayStatics.GetPlayerCharacter` 0)))
      (`/Game/Blueprints/BPC_PlayerStats.Increase XP` (`/Game/ThirdPerson/Blueprints/BP_ThirdPersonCharacter.BPC_PlayerStats` _asbp_third_person_character) 50.0))
    (:`then_1`
      (`KismetSystemLibrary.Delay` 3.0)
      (`self.K2_DestroyActor`))))

(event `Sword Trace Loop`
  ;[0.05127 0.05127 0.05127] Sword Trace
  (bind (_outhit _returnvalue) (`KismetSystemLibrary.SphereTraceSingle` :`Start` (`SceneComponent.K2_GetComponentLocation` (`self.Sword Top Point`)) :`End` (`SceneComponent.K2_GetComponentLocation` (`self.Sword Bottom Point`)) :`Radius` 25.0 :`TraceChannel` "TraceTypeQuery1" :`DrawTime` 2.0))
  (if _returnvalue
    (bind (_bblockinghit _binitialoverlap _time _distance _location _impactpoint _normal _impactnormal _physmat _hitactor) (`GameplayStatics.BreakHitResult` _outhit))
    (if (`self.ActorHasTag` _hitactor "Damageable")
      (`/Engine/EditorBlueprintResources/StandardMacros.DoOnce` false :!label _label
        (:`Completed`
          (`GameplayStatics.ApplyDamage` _hitactor 30.0)
          (`self.Sword SFX`)
          (`GameplayStatics.SpawnEmitterAtLocation` "/Game/FXs/Particles/Blood/P_Blood_Splat_Cone.P_Blood_Splat_Cone" _location (`KismetMathLibrary.MakeRotFromXY` _normal _normal) (0.4 0.4 0.4) true "AutoRelease")
          (`KismetSystemLibrary.Delay` 0.5)
          (goto _label :!via `Reset`))))))

(event `Ragdoll`
  ;[0.05127 0.05127 0.05127] Ragdoll
  (`KismetSystemLibrary.Delay` 2.0)
  (`GameplayStatics.PlaySoundAtLocation` "/Game/Audio/Grunts-Hit/SC_Death.SC_Death" (`SceneComponent.K2_GetComponentLocation` (`self.Mesh`)) (struct) 1.0 1.0 0.0 null null null null)
  (`KismetSystemLibrary.Delay` 0.5)
  (`CharacterMovementComponent.SetMovementMode` (`self.CharacterMovement`) "MOVE_None" 0)
  (`PrimitiveComponent.SetSimulatePhysics` (`self.Mesh`) true)
  (`KismetSystemLibrary.Delay` 3.0)
  (`self.K2_DestroyActor`))

(event `self.Assassination Radius.OnComponentBeginOverlap`
  (params (OverlappedComponent :type "PrimitiveComponent Object Reference") (OtherActor :type "Actor Object Reference") (OtherComp :type "PrimitiveComponent Object Reference") (OtherBodyIndex :type Integer) (bFromSweep :type Boolean) (SweepResult :type "HitResult Structure (by ref)"))
  ;[0.05127 0.05127 0.05127] Set Takedown Widget Visibility
  (cast `/Game/ThirdPerson/Blueprints/BP_ThirdPersonCharacter` OtherActor)
  (`SceneComponent.SetVisibility` (`self.Assassinate Widget`) true false))

(event `Stop Sword Trace`
  ;[0.05127 0.05127 0.05127] Sword Trace
  (`KismetSystemLibrary.K2_ClearAndInvalidateTimerHandle` (`self.swordTraceLoop`)))

(event `self.Assassinate Widget.OnComponentEndOverlap`
  (params (OverlappedComponent :type "PrimitiveComponent Object Reference") (OtherActor :type "Actor Object Reference") (OtherComp :type "PrimitiveComponent Object Reference") (OtherBodyIndex :type Integer))
  ;[0.05127 0.05127 0.05127] Set Takedown Widget Visibility
  (cast `/Game/ThirdPerson/Blueprints/BP_ThirdPersonCharacter` OtherActor)
  (`SceneComponent.SetVisibility` (`self.Assassinate Widget`) false false))

(event `Sword SFX`
  (`GameplayStatics.PlaySoundAtLocation` "/Game/Audio/Grunts-Hit/MS_SwordHit.MS_SwordHit" (`self.K2_GetActorLocation` (`self.GetOwner`)) (struct) 1.0 1.0 0.0 null null null null))

(event `self.ReceiveAnyDamage`
  (params (Damage :type "Float (single-precision)") (DamageType :type "DamageType Object Reference") (InstigatedBy :type "Controller Object Reference") (DamageCauser :type "Actor Object Reference"))
  ;[0.05127 0.05127 0.05127] Apply Damage
  (`self.PlayAnimMontage` (`|GetArrayItem` (`self.hitAnims`) (`KismetMathLibrary.RandomIntegerInRange` 0 (- (`KismetArrayLibrary.Array_Length` (`self.hitAnims`)) 1))))
  (bind _asbp_third_person_character (cast `/Game/ThirdPerson/Blueprints/BP_ThirdPersonCharacter` (`GameplayStatics.GetPlayerCharacter` 0)))
  (`self.LaunchCharacter` (* (`KismetMathLibrary.GetForwardVector` (`self.K2_GetActorRotation` _asbp_third_person_character)) 700.0))
  (`GameplayStatics.PlaySoundAtLocation` "/Game/Audio/Grunts-Hit/SC_Death.SC_Death" (`self.K2_GetActorLocation`) (struct) 1.0 1.0 0.0 "/Game/Audio/SA_Character.SA_Character" null null null)
  (bind _isplayerdead_ (`/Game/Blueprints/BPC_PlayerStats.Decrease Health` (`self.BPC_PlayerStats`) Damage))
  (if _isplayerdead_
    (`self.Die`)))

(event `Sphere Trace`
  (bind _returnvalue (`SceneComponent.K2_GetComponentLocation` (`self.Sphere Trace POS`)))
  ;[0.05127 0.05127 0.05127] Sphere Trace
  (bind (_outhit _returnvalue_2) (`KismetSystemLibrary.SphereTraceSingle` :`Start` _returnvalue :`End` _returnvalue :`Radius` 25.0 :`TraceChannel` "TraceTypeQuery1" :`DrawTime` 2.0))
  (if _returnvalue_2
    (bind (_bblockinghit _binitialoverlap _time _distance _location _impactpoint _normal _impactnormal _physmat _hitactor) (`GameplayStatics.BreakHitResult` _outhit))
    (if (`self.ActorHasTag` _hitactor "Damageable")
      (`GameplayStatics.ApplyDamage` _hitactor 30.0)
      (`self.Sword SFX`)
      (`GameplayStatics.SpawnEmitterAtLocation` "/Game/FXs/Particles/Blood/P_Blood_Splat_Cone.P_Blood_Splat_Cone" _location (`KismetMathLibrary.MakeRotFromXY` _normal _normal) (0.4 0.4 0.4) true "AutoRelease"))))

(event `SwordAttack_BT`
  ;[0.05127 0.05127 0.05127] Combo System
  ;;[0.05127 0.05127 0.05127] Attack Input
  (if (`self.canAttack?`)
    (`self.Sword Attack`)))

(event `Attack 1`
  ;[0.05127 0.05127 0.05127] Combo System
  ;;[0.05127 0.05127 0.05127] Attack 1
  (`/Engine/EditorBlueprintResources/StandardMacros.DoOnce` false :!label _label_2
    (:`Completed`
      (`KismetSystemLibrary.Delay` 0.1)
      (`|PlayMontage` (`self.Mesh`) "/Game/Characters/RPG_Character/Animations/SwordAttacks/Attack1_Montage.Attack1_Montage"
        (:`then`
          (set `self.attackIndex` 1)
          (goto _label_2 :!via `Reset`))))))

(event `Sword Attack`
  ;[0.05127 0.05127 0.05127] Combo System
  ;;[0.05127 0.05127 0.05127] Sword Attack
  (if (`self.isAttacking?`)
    (set `self.saveAttack?` true)
    (else
      (set `self.isAttacking?` true)
      (switch `int` (`self.attackIndex`) :!label _label_3
        (:`0`
          (`self.Attack 1`))
        (:`1`
          (`self.Attack 2`))
        (:`2`
          (`self.Attack 3`))))))

(event `Attack 2`
  ;[0.05127 0.05127 0.05127] Combo System
  ;;[0.05127 0.05127 0.05127] Attack 2
  (`/Engine/EditorBlueprintResources/StandardMacros.DoOnce` false :!label _label_4
    (:`Completed`
      (`KismetSystemLibrary.Delay` 0.1)
      (`|PlayMontage` (`self.Mesh`) "/Game/Characters/RPG_Character/Animations/SwordAttacks/Attack2_Montage.Attack2_Montage"
        (:`then`
          (set `self.attackIndex` 2)
          (goto _label_4 :!via `Reset`))))))

(event `Sword Attack Combo`
  ;[0.05127 0.05127 0.05127] Combo System
  ;;[0.05127 0.05127 0.05127] Combo Controller
  (if (`self.saveAttack?`)
    (set `self.saveAttack?` false)
    (goto _label_3)
    (else
      (`self.Stop Combo`))))

(event `Attack 3`
  ;[0.05127 0.05127 0.05127] Combo System
  ;;[0.05127 0.05127 0.05127] Attack 3
  (`/Engine/EditorBlueprintResources/StandardMacros.DoOnce` false :!label _label_5
    (:`Completed`
      (`KismetSystemLibrary.Delay` 0.1)
      (`|PlayMontage` (`self.Mesh`) "/Game/Characters/RPG_Character/Animations/SwordAttacks/Attack3_Montage.Attack3_Montage"
        (:`then`
          (set `self.attackIndex` 0)
          (goto _label_5 :!via `Reset`))))))

(event `Stop Combo`
  ;[0.05127 0.05127 0.05127] Combo System
  ;;[0.05127 0.05127 0.05127] Stop Combo
  (set `self.isAttacking?` false)
  (set `self.attackIndex` 0))

(fn `Attack`
  (returns (`Animation Duration` :type "Float (double-precision)"))
  (`self.SwordAttack_BT`)
  (return 0.4))

(fn `Stealth Back Assassination`
  (returns (`REF Location` :type "Vector Structure") (`Assassin Rotation` :type "Rotator Structure"))
  ;[1 1 1] Play Victim Montage
  (`self.PlayAnimMontage` "/Game/Characters/RPG_Character/Animations/Takedowns/Paired_Knife_Stealth_KidneyAndNeck_Vic_Montage.Paired_Knife_Stealth_KidneyAndNeck_Vic_Montage")
  (`self.Ragdoll`)
  (`SceneComponent.SetVisibility` (`self.Assassinate Widget`) false false)
  (return (`SceneComponent.K2_GetComponentLocation` (`self.Assassin REF`)) (`self.K2_GetActorRotation`)))

(fn `UserConstructionScript`)